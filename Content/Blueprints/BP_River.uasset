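; BP_River is a water hazard that drowns the chicken character when it enters without standing on a log or leaf.
; On Box overlap, it casts to BP_Chicken and checks its OnLog and OnLeaf flags.
; If both are false, it drops the chicken to a fixed sunken height, sets its CurrentPos to the river's own location and raises its DeathByDrowning flag.
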(event `self.Box.OnComponentBeginOverlap`
  (params (OverlappedComponent :type "PrimitiveComponent Object Reference") (OtherActor :type "Actor Object Reference") (OtherComp :type "PrimitiveComponent Object Reference") (OtherBodyIndex :type Integer) (bFromSweep :type Boolean) (SweepResult :type "HitResult Structure (by ref)"))
  (bind _asbp_chicken (cast `/Game/Blueprints/BP_Chicken` OtherActor))
  (if (not (or (`/Game/Blueprints/BP_Chicken.on log` _asbp_chicken) (`/Game/Blueprints/BP_Chicken.on leaf` _asbp_chicken)))
    (bind (_returnvalue_x _returnvalue_y) (`KismetMathLibrary.BreakVector` (`self.K2_GetActorLocation` _asbp_chicken)))
    (`self.K2_SetActorLocation` _asbp_chicken (`KismetMathLibrary.MakeVector` _returnvalue_x _returnvalue_y -50.0) false false)
    (set `/Game/Blueprints/BP_Chicken.current pos` (`self.K2_GetActorLocation`) _asbp_chicken)
    (set `/Game/Blueprints/BP_Chicken.death by drowning` true _asbp_chicken)))

(fn `UserConstructionScript`
  (`parent.UserConstructionScript`))