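; BP_Rail_road_sign is a railroad sign that switches on two warning lights as trains pass.
; BoxRight responds only to BP_Train_left and BoxLeft only to BP_Train_right.
; On overlap begin, the lights toggle in a short staggered sequence, mirrored per side, then both stay visible.
; On overlap end, both lights are hidden.
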(event `self.BoxRight.OnComponentBeginOverlap`
  (params (OverlappedComponent :type "PrimitiveComponent Object Reference") (OtherActor :type "Actor Object Reference") (OtherComp :type "PrimitiveComponent Object Reference") (OtherBodyIndex :type Integer) (bFromSweep :type Boolean) (SweepResult :type "HitResult Structure (by ref)"))
  (cast `/Game/Blueprints/BP_Train_left` OtherActor)
  (`SceneComponent.ToggleVisibility` (`self.PointLight1`) false)
  (`KismetSystemLibrary.Delay` 0.1)
  (`SceneComponent.ToggleVisibility` (`self.PointLight`) false)
  (`KismetSystemLibrary.Delay` 0.4)
  (`SceneComponent.SetVisibility` (`self.PointLight`) true false)
  (`SceneComponent.SetVisibility` (`self.PointLight1`) true false))

(event `self.BoxRight.OnComponentEndOverlap`
  (params (OverlappedComponent :type "PrimitiveComponent Object Reference") (OtherActor :type "Actor Object Reference") (OtherComp :type "PrimitiveComponent Object Reference") (OtherBodyIndex :type Integer))
  (cast `/Game/Blueprints/BP_Train_left` OtherActor)
  (`SceneComponent.SetVisibility` (`self.PointLight`) false false)
  (`SceneComponent.SetVisibility` (`self.PointLight1`) false false))

(event `self.BoxLeft.OnComponentBeginOverlap`
  (params (OverlappedComponent :type "PrimitiveComponent Object Reference") (OtherActor :type "Actor Object Reference") (OtherComp :type "PrimitiveComponent Object Reference") (OtherBodyIndex :type Integer) (bFromSweep :type Boolean) (SweepResult :type "HitResult Structure (by ref)"))
  (cast `/Game/Blueprints/BP_Train_right` OtherActor)
  (`SceneComponent.ToggleVisibility` (`self.PointLight`) false)
  (`KismetSystemLibrary.Delay` 0.1)
  (`SceneComponent.ToggleVisibility` (`self.PointLight1`) false)
  (`KismetSystemLibrary.Delay` 0.4)
  (`SceneComponent.SetVisibility` (`self.PointLight`) true false)
  (`SceneComponent.SetVisibility` (`self.PointLight1`) true false))

(event `self.BoxLeft.OnComponentEndOverlap`
  (params (OverlappedComponent :type "PrimitiveComponent Object Reference") (OtherActor :type "Actor Object Reference") (OtherComp :type "PrimitiveComponent Object Reference") (OtherBodyIndex :type Integer))
  (cast `/Game/Blueprints/BP_Train_right` OtherActor)
  (`SceneComponent.SetVisibility` (`self.PointLight`) false false)
  (`SceneComponent.SetVisibility` (`self.PointLight1`) false false))

(fn `UserConstructionScript`
  (`parent.UserConstructionScript`))