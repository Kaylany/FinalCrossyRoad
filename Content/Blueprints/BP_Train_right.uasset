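; BP_Train_right is a moving train hazard that kills the chicken on contact.
; Tick moves it along its local X axis with a swept offset scaled by TrainSpeed and delta time, then destroys it past a fixed world Y limit.
; Its Box overlap casts to BP_Chicken and, if not already hit, stores the chicken's position in CurrentPos and sets DeathByVehicle.
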(event `self.ReceiveTick`
  (params (DeltaSeconds :type "Float (single-precision)"))
  (bind (_returnvalue_x _returnvalue_y) (`KismetMathLibrary.BreakVector` (`self.K2_GetActorLocation` self)))
  (`self.K2_AddActorLocalOffset` (`KismetMathLibrary.MakeVector` (* DeltaSeconds (`self.train speed`))) true)
  (if (> _returnvalue_y 5000.0)
    (`self.K2_DestroyActor` self)))

(event `self.Box.OnComponentBeginOverlap`
  (params (OverlappedComponent :type "PrimitiveComponent Object Reference") (OtherActor :type "Actor Object Reference") (OtherComp :type "PrimitiveComponent Object Reference") (OtherBodyIndex :type Integer) (bFromSweep :type Boolean) (SweepResult :type "HitResult Structure (by ref)"))
  (bind _asbp_chicken (cast `/Game/Blueprints/BP_Chicken` OtherActor))
  (if (not (`/Game/Blueprints/BP_Chicken.death by vehicle` _asbp_chicken))
    (set `/Game/Blueprints/BP_Chicken.current pos` (`self.K2_GetActorLocation` _asbp_chicken) _asbp_chicken)
    (set `/Game/Blueprints/BP_Chicken.death by vehicle` true _asbp_chicken)))

(fn `UserConstructionScript`)