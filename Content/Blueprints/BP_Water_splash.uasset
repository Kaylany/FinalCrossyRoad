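; BP_Water_splash is a water splash actor tied to a Chicken reference, which sinks and removes itself once that reference is invalid.
; While Chicken is valid, Tick only records its location in CurrentPos.
; Otherwise, Tick moves the actor down at constant speed unless StartEffect is set.
; Below a Z threshold it destroys itself and sets StartEffect; above it, a two-second Delay clears the flag.
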(event `self.ReceiveTick`
  (params (DeltaSeconds :type "Float (single-precision)"))
  (bind (_returnvalue_x _returnvalue_y _returnvalue_z) (`KismetMathLibrary.BreakVector` (`self.K2_GetActorLocation`)))
  (bind _chicken (`self.chicken`))
  (`/Engine/EditorBlueprintResources/StandardMacros.IsValid` _chicken
    (:`Is Valid`
      (set `self.current pos` (`self.K2_GetActorLocation` _chicken)))
    (:`Is Not Valid`
      (`self.K2_AddActorLocalOffset` (`KismetMathLibrary.MakeVector` 0.0 0.0 (select `bool` (`self.start effect`) :`false` (* DeltaSeconds -160.0) :`true` (* DeltaSeconds 0.0))))
      (if (< _returnvalue_z -250.0)
        (`self.K2_DestroyActor`)
        (set `self.start effect` true)
        (else
          (`KismetSystemLibrary.Delay` 2.0)
          (set `self.start effect` false))))))

(fn `UserConstructionScript`)